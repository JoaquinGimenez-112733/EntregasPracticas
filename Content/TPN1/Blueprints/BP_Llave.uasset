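; BP_Llave is a key pickup that unlocks once every key fragment in the level has been collected.
; On BeginPlay it counts all BP_ItemFragmentoLlave actors and binds to their collected events, activating immediately if the counts already match.
; Each event increments the collected count and calls ActivarLlave when it reaches the total.
; Interacting sets TieneLlave on an actor without a key, then deactivates this key.
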(event `self.ReceiveBeginPlay`
  (`self.BindearFragmentos`)
  (if (== (`self.CantidadDeFragmentosTotales`) (`self.CantidadDeFragmentosRecolectados`))
    (`self.ActivarLlave`)))

(event `FragmentoRecolectado`
  (bind _cantidaddefragmentosrecolectados (`self.CantidadDeFragmentosRecolectados`))
  (`/Engine/EditorBlueprintResources/StandardMacros.IncrementInt` _cantidaddefragmentosrecolectados
    (:`  `
      (if (== (`self.CantidadDeFragmentosTotales`) _cantidaddefragmentosrecolectados)
        (`self.ActivarLlave`)))))

(event `/Game/TPN1/Interfaces/BPI_Interactuar.Interactuar`
  (params (Actor :type "/Game/ThirdPerson/Blueprints/BP_ThirdPersonCharacter Object Reference"))
  (if (not (`/Game/ThirdPerson/Blueprints/BP_ThirdPersonCharacter.bTieneLlave` Actor))
    (set `/Game/ThirdPerson/Blueprints/BP_ThirdPersonCharacter.bTieneLlave` true Actor)
    (`self.DesactivarLlave`)))

(fn `BindearFragmentos`
  (bind _outactors (`GameplayStatics.GetAllActorsOfClass` "/Game/TPN1/Blueprints/BP_ItemFragmentoLlave.BP_ItemFragmentoLlave_C"))
  (set `self.CantidadDeFragmentosTotales` (`KismetArrayLibrary.Array_Length` _outactors))
  (for _array_element _outactors
    (add `/Game/TPN1/Blueprints/BP_ItemFragmentoLlave.OnFragmentoRecolectado` _array_element (`|CreateDelegate` :!event `FragmentoRecolectado`))))

(fn `UserConstructionScript`)