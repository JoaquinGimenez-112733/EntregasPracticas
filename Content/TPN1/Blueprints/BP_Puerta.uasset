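; BP_Puerta is a double door that opens when the interacting actor has the key.
; The Interactuar event checks TieneLlave, printing a Spanish message to return with the key if it is missing.
; An Abierta flag limits opening to once, and a Timeline slides HojaIzquierda and HojaDerecha along X.
; Each update adds the track values to the leaves' current relative X, so the offsets accumulate rather than interpolate between fixed positions.
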(event `/Game/TPN1/Interfaces/BPI_Interactuar.Interactuar`
  (params (Actor :type "/Game/ThirdPerson/Blueprints/BP_ThirdPersonCharacter Object Reference"))
  (bind _hojaderecha (`self.HojaDerecha`))
  (bind _hojaizquierda (`self.HojaIzquierda`))
  (bind _relativelocation_x (`KismetMathLibrary.BreakVector` (`SceneComponent.RelativeLocation` _hojaderecha)))
  (bind _relativelocation_x_2 (`KismetMathLibrary.BreakVector` (`SceneComponent.RelativeLocation` _hojaizquierda)))
  (if (`/Game/ThirdPerson/Blueprints/BP_ThirdPersonCharacter.bTieneLlave` Actor)
    (if (not (`self.bAbierta`))
      (set `self.bAbierta` true)
      (bind (_direction _izquierda _derecha) (`Timeline|Timeline`)
        (:`Update`
          (`SceneComponent.K2_SetRelativeLocation` _hojaizquierda (`KismetMathLibrary.MakeVector` (+ _relativelocation_x_2 _izquierda)) false false)
          (`SceneComponent.K2_SetRelativeLocation` _hojaderecha (`KismetMathLibrary.MakeVector` (+ _relativelocation_x _derecha)) false false))))
    (else
      (`KismetSystemLibrary.PrintString` "Volve cuando tengas la llave maestro"))))

(fn `UserConstructionScript`)